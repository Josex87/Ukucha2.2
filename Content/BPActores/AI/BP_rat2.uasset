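; Rat character for an operant-conditioning experiment, performing animated behaviors like begging, grooming, rolling and lever pressing.
; Each behavior checks for food (reward) or a key-triggered shock (punishment), adjusts its learning counter, then POSTs the result via VaRest.
; Next-action logic randomly evaluates counter thresholds, drinks or casts to Rata_AI.
; Threshold branches only log or label learned actions; BeginPlay is empty and nothing follows the cast.
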(event `Grabar datos-Ukucha`
  ;[1 1 1 1 40] Manejo de datos
  (`KismetSystemLibrary.PrintString` "Guardando datos")
  (bind _asuku_game_instance (cast `/Game/Widgets/Uku_GameInstance` (`GameplayStatics.GetGameInstance`)))
  (bind _target (`|MakeJson` (`KismetMathLibrary.Conv_IntToDouble` (`/Game/Widgets/Uku_GameInstance.codigoExperimento` _asuku_game_instance)) (`self.acciónRata`) (`self.recompensaCastigo`)))
  (`KismetSystemLibrary.PrintString` (`KismetSystemLibrary.GetDisplayName` _target))
  (`VaRestSubsystem.CallURL` (subsystem `VaRestSubsystem`) "https://ukuchacorp.herokuapp.com/rata/api/detalles/" "POST" "json" _target (delegate `RestCallback`)))

(event `InputAction|Electrocutar`
  (params (Key :type "Key Structure"))
  ;[1 1 1] Tecla electrocutar
  (:`Pressed`
    (`KismetSystemLibrary.PrintString` (`KismetTextLibrary.Conv_TextToString` (`KismetInputLibrary.Key_GetDisplayName` Key)))
    (set `self.¿Se electrocuta?` true)
    (`KismetSystemLibrary.PrintString` "Electrocutada")))

(event `self.ReceiveBeginPlay`
  ;[1 1 1] Iniciar
)

(event `RestCallback`
  (params (Request :type "VaRestRequestJSON Object Reference"))
  ;[1 1 1 1 40] Manejo de datos
  (if (`KismetStringLibrary.EqualEqual_StrStr` (`VaRestJsonObject.GetStringField` (`VaRestRequestJSON.GetResponseObject` Request) "Message") "Ok")
    (`KismetSystemLibrary.PrintString` "Datos guardados")
    (else
      (`KismetSystemLibrary.PrintString` "Datos sin guardar"))))

(event `LimpiarCabeza-Ukucha`
  ;[1 1 1] Limpiar cabeza
  (`self.Stop animation`)
  (`self.Play animation` "/Game/modelo-ukucha/animaciones/limpiar-cabeza_Armature_limpiar-cabeza.limpiar-cabeza_Armature_limpiar-cabeza" true)
  (set `self.acciónRata` "Rata limpiando su cara")
  (`KismetSystemLibrary.Delay` 2.46)
  (bind _asuku_game_instance (cast `/Game/Widgets/Uku_GameInstance` (`GameplayStatics.GetGameInstance`)))
  (if (`/Game/Widgets/Uku_GameInstance.ComidaExiste` _asuku_game_instance)
    (`self.Comiendo-Ukucha`)
    (set `self.prbLimpiarseCara` (+ (`self.prbLimpiarseCara`) 1))
    (else
      (if (`self.¿Se electrocuta?`)
        (`self.Electrocutar-Ukucha`)
        (set `self.¿Se electrocuta?` false)
        (else
          (set `self.recompensaCastigo` "Sin acción")))
      (set `self.prbLimpiarseCara` (- (`self.prbLimpiarseCara`) 1))))
  (`self.Grabar datos-Ukucha`)
  (`self.DecidirAccionSiguiente-Ukucha` true))

(event `Rodar-Ukucha`
  ;[1 1 1] Rodar
  (`self.Stop animation`)
  (`self.Play animation` "/Game/modelo-ukucha/animaciones/rodar.rodar" true)
  (`|AIMoveTo` self (`NavigationSystemV1.K2_GetRandomReachablePointInRadius` (`self.K2_GetActorLocation`) 15000.0 null null) null
    (:`OnSuccess`
      (set `self.acciónRata` "Rata rodando")
      (bind _asuku_game_instance (cast `/Game/Widgets/Uku_GameInstance` (`GameplayStatics.GetGameInstance`)))
      (if (`/Game/Widgets/Uku_GameInstance.ComidaExiste` _asuku_game_instance)
        (`self.Comiendo-Ukucha`)
        (set `self.prbRodar` (+ (`self.prbRodar`) 1))
        (else
          (if (`self.¿Se electrocuta?`)
            (`self.Electrocutar-Ukucha`)
            (set `self.¿Se electrocuta?` false)
            (else
              (set `self.recompensaCastigo` "Sin acción")))
          (set `self.prbRodar` (- (`self.prbRodar`) 1))))
      (`self.Grabar datos-Ukucha`)
      (`self.DecidirAccionSiguiente-Ukucha` true))))

(event `Esconder Cara-Ukucha`
  ;[1 1 1] Esconder Cara
  (`self.Stop animation`)
  (`self.Play animation` "/Game/modelo-ukucha/animaciones/esconder-cabeza_Armature_Esconder-la-cabeza.esconder-cabeza_Armature_Esconder-la-cabeza" true)
  (set `self.acciónRata` "Rata escondiendo su cara")
  (`KismetSystemLibrary.Delay` 1.83)
  (bind _asuku_game_instance (cast `/Game/Widgets/Uku_GameInstance` (`GameplayStatics.GetGameInstance`)))
  (if (`/Game/Widgets/Uku_GameInstance.ComidaExiste` _asuku_game_instance)
    (`self.Comiendo-Ukucha`)
    (set `self.prbEsconderCara` (+ (`self.prbEsconderCara`) 1))
    (else
      (if (`self.¿Se electrocuta?`)
        (`self.Electrocutar-Ukucha`)
        (set `self.¿Se electrocuta?` false)
        (else
          (set `self.recompensaCastigo` "Sin acción")))
      (set `self.prbEsconderCara` (- 0 (`self.prbEsconderCara`)))))
  (`self.Grabar datos-Ukucha`)
  (`self.DecidirAccionSiguiente-Ukucha` true))

(event `LimpiarCuerpo-Ukucha`
  ;[1 1 1] Limpiar cuerpo
  (`self.Stop animation`)
  (`self.Play animation` "/Game/modelo-ukucha/animaciones/Limpiarcuerpo2.Limpiarcuerpo2" true)
  (set `self.acciónRata` "Rata limpiando su cuerpo")
  (`KismetSystemLibrary.Delay` 10.38)
  (bind _asuku_game_instance (cast `/Game/Widgets/Uku_GameInstance` (`GameplayStatics.GetGameInstance`)))
  (if (`/Game/Widgets/Uku_GameInstance.ComidaExiste` _asuku_game_instance)
    (`self.Comiendo-Ukucha`)
    (set `self.prbLimpiarseCuerpo` (+ (`self.prbLimpiarseCuerpo`) 1))
    (else
      (if (`self.¿Se electrocuta?`)
        (`self.Electrocutar-Ukucha`)
        (set `self.¿Se electrocuta?` false)
        (else
          (set `self.recompensaCastigo` "Sin acción")))
      (set `self.prbLimpiarseCuerpo` (- (`self.prbLimpiarseCuerpo`) 1))))
  (`self.Grabar datos-Ukucha`)
  (`self.DecidirAccionSiguiente-Ukucha` true))

(event `DecidirAccionSiguiente-Ukucha`
  (params (saltarDelay :type Boolean) (Target :type "/Game/BPActores/AI/BP_rat2 Object Reference"))
  ;[1 1 1] Decidir siguiente accion
  (bind _asuku_game_instance (cast `/Game/Widgets/Uku_GameInstance` (`GameplayStatics.GetGameInstance`)))
  (bind _output_get (set `/Game/Widgets/Uku_GameInstance.ComidaExiste` false _asuku_game_instance))
  (bind _output_get_2 (set `self.¿Se electrocuta?` false))
  (`KismetSystemLibrary.PrintString` (`KismetStringLibrary.Concat_StrStr` "Existe comida" (`KismetStringLibrary.Conv_BoolToString` _output_get) "Electro" (`KismetStringLibrary.Conv_BoolToString` _output_get_2)))
  (if saltarDelay
    (if (`KismetMathLibrary.RandomBool`)
      (`self.Elegirvalor100`)
      (switch `int` (`/Game/BPActores/AI/BP_rat2.Acción` Target)
        (:`0`
          (`KismetSystemLibrary.PrintString` "Rogando")
          (`self.Probabilidades-Ukucha`))
        (:`1`
          (`KismetSystemLibrary.PrintString` "Limpiarcara")
          (`self.Probabilidades-Ukucha`))
        (:`2`
          (`KismetSystemLibrary.PrintString` "Limpiarcuerpo")
          (`self.Probabilidades-Ukucha`))
        (:`3`
          (`KismetSystemLibrary.PrintString` "Escondercara")
          (`self.Probabilidades-Ukucha`))
        (:`4`
          (`KismetSystemLibrary.PrintString` "TocarPalanca")
          (`self.Probabilidades-Ukucha`))
        (:`5`
          (set `/Game/BPActores/AI/BP_rat2.recompensaCastigo` "Acción aprendida" Target)
          (set `/Game/BPActores/AI/BP_rat2.acciónRata` (`/Game/BPActores/AI/BP_rat2.AccionReforzada` Target) Target)))
      (elif (`KismetMathLibrary.RandomBool`)
        (`self.Beber-Ukucha`)
        (else
          (cast `/Game/BPActores/AI/Rata_AI` (`self.GetController`) :!label _label))))
    (else
      (`KismetSystemLibrary.Delay` 2.0)
      (goto _label))))

(event `Probabilidades-Ukucha`
  ;[1 1 1] Decidir siguiente accion
  (`KismetSystemLibrary.PrintString` (`KismetStringLibrary.Concat_StrStr` "Rodar" (`KismetStringLibrary.Conv_IntToString` (`/Game/BPActores/AI/BP_rat2.prbRodar` (stale `DecidirAccionSiguiente-Ukucha` Target))) "Rogar" (`KismetStringLibrary.Conv_IntToString` (`/Game/BPActores/AI/BP_rat2.prbRogar` (stale `DecidirAccionSiguiente-Ukucha` Target))) "Cuerpo" (`KismetStringLibrary.Conv_IntToString` (`/Game/BPActores/AI/BP_rat2.prbLimpiarseCuerpo` (stale `DecidirAccionSiguiente-Ukucha` Target))) "Cara" (`KismetStringLibrary.Conv_IntToString` (`/Game/BPActores/AI/BP_rat2.prbLimpiarseCara` (stale `DecidirAccionSiguiente-Ukucha` Target))) "Palanca" (`KismetStringLibrary.Conv_IntToString` (`/Game/BPActores/AI/BP_rat2.prbTocarPalanca` (stale `DecidirAccionSiguiente-Ukucha` Target))) "Esconder" (`KismetStringLibrary.Conv_IntToString` (`/Game/BPActores/AI/BP_rat2.prbEsconderCara` (stale `DecidirAccionSiguiente-Ukucha` Target)))))
  (bind _asuku_game_instance (cast `/Game/Widgets/Uku_GameInstance` (`GameplayStatics.GetGameInstance`)))
  (`KismetSystemLibrary.PrintString` (`KismetStringLibrary.Concat_StrStr` "Electro:" (`KismetStringLibrary.Conv_BoolToString` (`self.¿Se electrocuta?`)) "Recompensa" (`self.recompensaCastigo`) "Existe:" (`KismetStringLibrary.Conv_BoolToString` (`/Game/Widgets/Uku_GameInstance.ComidaExiste` _asuku_game_instance)))))

(event `Rogar-Ukucha`
  ;[1 1 1] Rogar
  (`self.Stop animation`)
  (`self.Play animation` "/Game/modelo-ukucha/animaciones/rogar_Armature_rogar.rogar_Armature_rogar" true)
  (set `self.acciónRata` "Rata rogando")
  (`KismetSystemLibrary.Delay` 3.71)
  (bind _asuku_game_instance (cast `/Game/Widgets/Uku_GameInstance` (`GameplayStatics.GetGameInstance`)))
  (if (`/Game/Widgets/Uku_GameInstance.ComidaExiste` _asuku_game_instance)
    (`self.Comiendo-Ukucha`)
    (set `self.prbRogar` (+ (`self.prbRogar`) 1))
    (else
      (if (`self.¿Se electrocuta?`)
        (`self.Electrocutar-Ukucha`)
        (set `self.¿Se electrocuta?` false)
        (else
          (set `self.recompensaCastigo` "Sin acción")))
      (set `self.prbRogar` (- (`self.prbRogar`) 1))))
  (`self.Grabar datos-Ukucha`)
  (`self.DecidirAccionSiguiente-Ukucha` true))

(event `Elegirvalor100`
  (bind _prbescondercara (`self.prbEsconderCara`))
  (bind _prbrogar (`self.prbRogar`))
  (bind _prblimpiarsecara (`self.prbLimpiarseCara`))
  (bind _prblimpiarsecuerpo (`self.prbLimpiarseCuerpo`))
  (bind _prbtocarpalanca (`self.prbTocarPalanca`))
  ;[1 1 1 1 40] Ajuste de probabilidades
  (if (and (>= _prbrogar 50) (< _prbrogar 100))
    (set `self.Acción` 0)
    (elif (== (`self.prbRogar`) 100)
      (set `self.Acción` 5)
      (set `self.AccionReforzada` "Rogar")
      (elif (and (>= _prblimpiarsecara 50) (< _prblimpiarsecara 100))
        (set `self.Acción` 1)
        (elif (== (`self.prbLimpiarseCara`) 100)
          (set `self.Acción` 5)
          (set `self.AccionReforzada` "Limpiarse la cara")
          (elif (and (>= _prblimpiarsecuerpo 50) (< _prblimpiarsecuerpo 100))
            (set `self.Acción` 2)
            (elif (== (`self.prbLimpiarseCuerpo`) 100)
              (set `self.Acción` 5)
              (set `self.AccionReforzada` "Limpiarse el cuerpo")
              (elif (and (>= _prbtocarpalanca 50) (< _prbtocarpalanca 100))
                (set `self.Acción` 3)
                (elif (== (`self.prbTocarPalanca`) 100)
                  (set `self.Acción` 5)
                  (set `self.AccionReforzada` "Limpiarse la cara")
                  (elif (and (>= _prbescondercara 50) (< _prbescondercara 100))
                    (set `self.Acción` 4)
                    (elif (== (`self.prbEsconderCara`) 100)
                      (set `self.Acción` 5)
                      (set `self.AccionReforzada` "Esconder la cara")
                      (else
                        (set `self.Acción` 5)))))))))))))

(event `TocarPalanca-Ukucha`
  ;[1 1 1] Tocar la palanca
  (`MovementComponent.StopMovementImmediately` (`self.CharacterMovement`))
  (if (> (`self.prbTocarPalanca`) 40)
    (`self.CaminarPalanca-Ukucha`)
    (`MovementComponent.StopMovementImmediately` (`self.CharacterMovement`))
    (`self.Play animation` "/Game/modelo-ukucha/animaciones/palanca_Armature_palanca.palanca_Armature_palanca")
    (set `self.acciónRata` "Rata tocando la palanca")
    (`KismetSystemLibrary.Delay` 2.92)
    (bind _asuku_game_instance (cast `/Game/Widgets/Uku_GameInstance` (`GameplayStatics.GetGameInstance`)))
    (if (`/Game/Widgets/Uku_GameInstance.ComidaExiste` _asuku_game_instance)
      (set `self.prbTocarPalanca` (+ (`self.prbTocarPalanca`) 1))
      (`self.Comiendo-Ukucha`)
      (else
        (if (`self.¿Se electrocuta?`)
          (`self.Electrocutar-Ukucha`)
          (set `self.¿Se electrocuta?` false)
          (else
            (set `self.recompensaCastigo` "Sin acción")))
        (set `self.prbTocarPalanca` (- (`self.prbTocarPalanca`) 1))))
    (`self.Grabar datos-Ukucha`)
    (`self.DecidirAccionSiguiente-Ukucha` false)
    (else
      (bind _asuku_game_instance_2 (cast `/Game/Widgets/Uku_GameInstance` (`GameplayStatics.GetGameInstance`))))))

(event `Beber-Ukucha`
  ;[1 1 1] Beber
  (`self.Stop animation`)
  (`self.CaminarBeber-Ukucha`)
  (`self.Play animation` "/Game/modelo-ukucha/animaciones/beber_Armature_beber.beber_Armature_beber")
  (`KismetSystemLibrary.Delay` 2.25)
  (`self.DecidirAccionSiguiente-Ukucha` false))

(event `Electrocutar`
  ;[1 1 1] Saltar/electrocutar
  (`self.Stop animation`)
  (`self.Play animation` "/Game/modelo-ukucha/animaciones/saltar_Armature_saltar.saltar_Armature_saltar" true)
  (`KismetSystemLibrary.Delay` 2.5))

(event `Electrocutar-Ukucha`
  ;[1 1 1] Electrocutar
  (`MovementComponent.StopMovementImmediately` (`self.CharacterMovement`))
  (`self.Play animation` "/Game/modelo-ukucha/animaciones/saltar_Armature_saltar.saltar_Armature_saltar" true)
  (set `self.recompensaCastigo` "Castigo")
  (`KismetSystemLibrary.Delay` 2.5))

(event `Comiendo-Ukucha`
  ;[1 1 1] Comiendo
  (`MovementComponent.StopMovementImmediately` (`self.CharacterMovement`))
  (`self.CaminarComida-Ukucha`)
  (`self.Play animation` "/Game/modelo-ukucha/AI/BP_comer.BP_comer")
  (`KismetSystemLibrary.Delay` 4.54)
  (set `self.recompensaCastigo` "Recompensa")
  (`MovementComponent.StopMovementImmediately` (`self.CharacterMovement`)))

(event `CaminarComida-Ukucha`
  ;[1 1 1] Caminar lugar de comida
  (`self.Stop animation`)
  (`self.Play animation` "/Game/modelo-ukucha/animaciones/caminar_Armature_caminar.caminar_Armature_caminar" true)
  (`|AIMoveTo` self (`self.Lugar de comida`) null 25.0 :!label _label_2
    (:`OnSuccess`
      (`KismetSystemLibrary.PrintString` "Funciona caminata a lugar de comida"))
    (:`OnFail`
      (`KismetSystemLibrary.PrintString` "No funcionó caminata a lugar de la comida")
      (goto _label_2))))

(event `CaminarPalanca-Ukucha`
  ;[1 1 1] Caminar al lugar de la palanca
  (`self.Stop animation`)
  (`self.Play animation` "/Game/modelo-ukucha/animaciones/caminar_Armature_caminar.caminar_Armature_caminar")
  (`|AIMoveTo` self (`self.Lugar de palanca`) null 25.0 :!label _label_3
    (:`OnSuccess`
      (`KismetSystemLibrary.PrintString` "Funciona caminata a lugar de la palanca"))
    (:`OnFail`
      (`KismetSystemLibrary.PrintString` "No funcionó caminata a lugar de la palanca")
      (goto _label_3))))

(event `CaminarBeber-Ukucha`
  ;[1 1 1] Caminar lugar de bebida
  (`self.Stop animation`)
  (`self.Play animation` "/Game/modelo-ukucha/animaciones/caminar_Armature_caminar.caminar_Armature_caminar" true)
  (`|AIMoveTo` self (`self.Lugar de bebida`) null 25.0 :!label _label_4
    (:`OnSuccess`
      (`KismetSystemLibrary.PrintString` "Funciona caminata a lugar de beber"))
    (:`OnFail`
      (`KismetSystemLibrary.PrintString` "No funcionó caminata a lugar de la comida")
      (goto _label_4))))

(fn `Play animation`
  (params (Animation :type "AnimationAsset Object Reference") (`Should loop?` :type Boolean))
  (`SkeletalMeshComponent.PlayAnimation` (`self.Mesh`) Animation `Should loop?`))

(fn `Stop animation`
  (bind _mesh (`self.Mesh`))
  (`SkeletalMeshComponent.SetAnimationMode` _mesh "AnimationBlueprint")
  (`SkeletalMeshComponent.SetAnimInstanceClass` _mesh null))

(fn `UserConstructionScript`)