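; Rat AI character that wanders, runs and performs animated behaviours such as grooming, begging, rolling and an electrocution jump.
; DecideNextAction starts on BeginPlay and loops through state flags to choose running, random walking or genital grooming; its random delay is bypassed.
; Events for walking to lever, food and drink spots retry failed moves, then play the matching animation without resuming the loop.
; Animations play directly on the mesh, with StopAnimation switching back to AnimationBlueprint mode.
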(event `Esconder Cara`
  ;[1 1 1] Esconder Cara
  (`self.Stop animation`)
  (`self.Play animation` "/Game/modelo-ukucha/animaciones/esconder-cabeza_Armature_Esconder-la-cabeza.esconder-cabeza_Armature_Esconder-la-cabeza" true)
  (`KismetSystemLibrary.Delay` 1.83)
  (`self.Decide Next Action` true))

(event `self.ReceiveBeginPlay`
  ;[1 1 1] Set up blueprint
  (`self.Decide Next Action` false))

(event `Beber`
  ;[1 1 1] Beber
  (`self.Stop animation`)
  (`self.Play animation` "/Game/modelo-ukucha/animaciones/beber_Armature_beber.beber_Armature_beber")
  (`KismetSystemLibrary.Delay` 2.25)
  (`self.Stop animation`))

(event `Decide Next Action`
  (params (`Skip delay?` :type Boolean))
  ;[1 1 1] Decide next action
  (if (not true)
    (`KismetSystemLibrary.Delay` (`KismetMathLibrary.Conv_IntToDouble` (`KismetMathLibrary.RandomIntegerInRange` 1 5))))
  (if (`self.Should Run?`)
    (`self.Correr`)
    (elif (`self.Is Hungry?`)
      (`self.Caminar Aleatoriamente`)
      (elif (`self.Is tired?`)
        (`self.Tocar genitales`)
        (else
          (`self.Caminar Aleatoriamente`))))))

(event `Rogar`
  ;[1 1 1] Rogar
  (`self.Stop animation`)
  (`self.Play animation` "/Game/modelo-ukucha/animaciones/rogar_Armature_rogar.rogar_Armature_rogar" true)
  (`KismetSystemLibrary.Delay` 3.71)
  (`self.Decide Next Action` true))

(event `Palanca`
  ;[1 1 1] Palanca
  (`self.Stop animation`)
  (`self.Play animation` "/Game/modelo-ukucha/animaciones/palanca_Armature_palanca.palanca_Armature_palanca" true)
  (`KismetSystemLibrary.Delay` 2.92)
  (`self.Stop animation`))

(event `Caminar Aleatoriamente`
  ;[1 1 1] Caminar aleatoriamente
  (set `CharacterMovementComponent.MaxWalkSpeed` 120.0 (`self.CharacterMovement`))
  (`|AIMoveTo` self (`NavigationSystemV1.K2_GetRandomReachablePointInRadius` (`self.K2_GetActorLocation`) 1500.0 null null) null
    (:`OnSuccess`
      (`self.Decide Next Action` false))))

(event `Tocar genitales`
  ;[1 1 1] Tocar genitales
  (`self.Stop animation`)
  (`self.Play animation` "/Game/modelo-ukucha/animaciones/tocar-genitales_Armature_tocar-genitales.tocar-genitales_Armature_tocar-genitales" true)
  (`KismetSystemLibrary.Delay` 3.29)
  (`self.Decide Next Action` true))

(event `LimpiarCabeza`
  ;[1 1 1] Limpiar cabeza
  (`self.Stop animation`)
  (`self.Play animation` "/Game/modelo-ukucha/animaciones/limpiar-cabeza_Armature_limpiar-cabeza.limpiar-cabeza_Armature_limpiar-cabeza")
  (`KismetSystemLibrary.Delay` 1.5)
  (`self.Decide Next Action` false))

(event `CaminarPalanca`
  ;[1 1 1] Caminar al lugar de la palanca
  (`self.Stop animation`)
  (`self.Play animation` "/Game/modelo-ukucha/animaciones/caminar_Armature_caminar.caminar_Armature_caminar" true)
  (`|AIMoveTo` self (`self.Lugar palanca`) null 25.0 :!label _label
    (:`OnSuccess`
      (`self.Palanca`))
    (:`OnFail`
      (`KismetSystemLibrary.PrintString` "No funcionó caminata a lugar de la palanca")
      (goto _label))))

(event `Correr`
  ;[1 1 1] Corrrer
  (set `CharacterMovementComponent.MaxWalkSpeed` 600.0 (`self.CharacterMovement`))
  (`|AIMoveTo` self (`NavigationSystemV1.K2_GetRandomReachablePointInRadius` (`self.K2_GetActorLocation`) (`KismetMathLibrary.RandomFloatInRange` 20000.0 30000.0) null null) null
    (:`OnSuccess`
      (`self.Decide Next Action` true))))

(event `Comer`
  ;[1 1 1] Comer
  (`self.Stop animation`)
  (`self.Play animation` "/Game/modelo-ukucha/animaciones/comer_Armature_comer.comer_Armature_comer" true)
  (`KismetSystemLibrary.Delay` 4.54)
  (`self.Stop animation`))

(event `LimpiarCuerpo`
  ;[1 1 1] Limpiar cuerpo
  (`self.Stop animation`)
  (`self.Play animation` "/Game/modelo-ukucha/animaciones/Limpiarcuerpo2.Limpiarcuerpo2" true)
  (`KismetSystemLibrary.Delay` 10.0)
  (`self.Decide Next Action` true))

(event `CaminarComida`
  ;[1 1 1] Caminar lugar de comida
  (`self.Stop animation`)
  (`self.Play animation` "/Game/modelo-ukucha/animaciones/caminar_Armature_caminar.caminar_Armature_caminar" true)
  (`|AIMoveTo` self (`self.Lugar comida`) null 25.0 :!label _label_2
    (:`OnSuccess`
      (`self.Comer`))
    (:`OnFail`
      (`KismetSystemLibrary.PrintString` "No funcionó caminata a lugar de la comida")
      (goto _label_2))))

(event `Electrocutar`
  ;[1 1 1] Saltar/electrocutar
  (`self.Stop animation`)
  (`self.Play animation` "/Game/modelo-ukucha/animaciones/saltar_Armature_saltar.saltar_Armature_saltar" true)
  (`KismetSystemLibrary.Delay` 2.0)
  (`self.Decide Next Action` true))

(event `Caminata`
  ;[1 1 1] otro ejemplo
  (`SkeletalMeshComponent.PlayAnimation` (`self.Mesh`) "/Game/modelo-ukucha/animaciones/caminar_Armature_caminar.caminar_Armature_caminar" true)
  (`|AIMoveTo` self (`NavigationSystemV1.K2_GetRandomLocationInNavigableRadius` (`self.K2_GetActorLocation` (`GameplayStatics.GetPlayerCharacter` 0)) 3000.0 null null) null
    (:`OnSuccess`
      (`SkeletalMeshComponent.Stop` (`self.Mesh`))
      (`KismetSystemLibrary.Delay` 0.2)
      (`self.Caminata`))))

(event `Rodar`
  ;[1 1 1] Rodar
  (`self.Stop animation`)
  (`self.Play animation` "/Game/modelo-ukucha/animaciones/rodar.rodar" true)
  (`|AIMoveTo` self (`NavigationSystemV1.K2_GetRandomReachablePointInRadius` (`self.K2_GetActorLocation`) 15000.0 null null) null
    (:`OnSuccess`
      (`self.Decide Next Action` true))))

(event `CaminarBebida`
  ;[1 1 1] Caminar lugar de bebida
  (`self.Stop animation`)
  (`self.Play animation` "/Game/modelo-ukucha/animaciones/caminar_Armature_caminar.caminar_Armature_caminar" true)
  (`|AIMoveTo` self (`self.Lugar bebida`) null 25.0 :!label _label_3
    (:`OnSuccess`
      (`self.Beber`))
    (:`OnFail`
      (`KismetSystemLibrary.PrintString` "No funcionó caminata a lugar de bebida")
      (goto _label_3))))

(fn `Play animation`
  (params (Animation :type "AnimationAsset Object Reference") (`Should loop?` :type Boolean))
  (`SkeletalMeshComponent.PlayAnimation` (`self.Mesh`) Animation `Should loop?`))

(fn `Stop animation`
  (bind _mesh (`self.Mesh`))
  (`SkeletalMeshComponent.SetAnimationMode` _mesh "AnimationBlueprint")
  (`SkeletalMeshComponent.SetAnimInstanceClass` _mesh null))

(fn `UserConstructionScript`)