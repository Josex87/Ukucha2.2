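; BP_Comida is a food actor that appears on player input and disappears when another actor overlaps it.
; It starts hidden with player input enabled; the DarComida action or D key shows it and sets ComidaExiste on Uku_GameInstance.
; The D key also plays the Palanca (lever) sound and sets ToquePalanca.
; Any overlap hides the food and clears ComidaExiste, and both inputs print the pressed key.
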(event `self.ReceiveActorBeginOverlap`
  (params (OtherActor :type "Actor Object Reference"))
  (`SceneComponent.SetVisibility` (`self.BP_Comida`) false false)
  (bind _asuku_game_instance (cast `/Game/Widgets/Uku_GameInstance` (`GameplayStatics.GetGameInstance`)))
  (set `/Game/Widgets/Uku_GameInstance.ComidaExiste` false _asuku_game_instance))

(event `self.ReceiveBeginPlay`
  (`SceneComponent.SetVisibility` (`self.BP_Comida`) false false)
  (`self.EnableInput` (`GameplayStatics.GetPlayerController` 0)))

(event `InputAction|DarComida`
  (params (Key :type "Key Structure"))
  (:`Pressed`
    (`KismetSystemLibrary.PrintString` (`KismetTextLibrary.Conv_TextToString` (`KismetInputLibrary.Key_GetDisplayName` Key)))
    (bind _asuku_game_instance (cast `/Game/Widgets/Uku_GameInstance` (`GameplayStatics.GetGameInstance`)))
    (set `/Game/Widgets/Uku_GameInstance.ComidaExiste` true _asuku_game_instance)
    (`SceneComponent.SetVisibility` (`self.BP_Comida`) true false)))

(event `Key|D`
  (params (Key :type "Key Structure"))
  (:`Pressed`
    (`KismetSystemLibrary.PrintString` (`KismetTextLibrary.Conv_TextToString` (`KismetInputLibrary.Key_GetDisplayName` Key)))
    (`GameplayStatics.PlaySoundAtLocation` "/Game/sonidos/SonidosWav/fbx_wav/Palanca.Palanca" (`self.K2_GetActorLocation`) (struct) 1.0 1.0 0.0 null null null)
    (bind _asuku_game_instance (cast `/Game/Widgets/Uku_GameInstance` (`GameplayStatics.GetGameInstance`)))
    (set `/Game/Widgets/Uku_GameInstance.toquePalanca` true _asuku_game_instance)
    (set `/Game/Widgets/Uku_GameInstance.ComidaExiste` true _asuku_game_instance)
    (`SceneComponent.SetVisibility` (`self.BP_Comida`) true false)))

(fn `UserConstructionScript`)