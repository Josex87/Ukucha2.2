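; BP_Ukucha is an AI-movable character with custom events for grooming head or body, rolling, and a jump/electrocute reaction.
; Each of those events resets the mesh through StopAnimation, then loops a clip via PlayAnimation.
; Rolling also sends it to a random reachable point, while head cleaning stops after a short delay.
; A random-animation event plays an array clip, then immediately calls StopAnimation; nothing here triggers these events.
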(event `LimpiarCabeza`
  ;[1 1 1] Limpiar cabeza
  (`self.Stop animation`)
  (`self.Play animation` "/Game/modelo-ukucha/animaciones/limpiar-cabeza_Armature_limpiar-cabeza.limpiar-cabeza_Armature_limpiar-cabeza" true)
  (`KismetSystemLibrary.Delay` 1.5)
  (`self.Stop animation`))

(event `Rodar`
  ;[1 1 1] Rodar
  (`self.Stop animation`)
  (`self.Play animation` "/Game/modelo-ukucha/animaciones/rodar.rodar" true)
  (`|AIMoveTo` self (`NavigationSystemV1.K2_GetRandomReachablePointInRadius` (`self.K2_GetActorLocation`) 30000.0 null null) null))

(event `LimpiarCuerpo`
  ;[1 1 1] Limpiar cuerpo
  (`self.Stop animation`)
  (`self.Play animation` "/Game/modelo-ukucha/animaciones/Limpiarcuerpo2.Limpiarcuerpo2" true))

(event `Electrocutar`
  ;[1 1 1] Saltar/electrocutar
  (`self.Stop animation`)
  (`self.Play animation` "/Game/modelo-ukucha/animaciones/saltar_Armature_saltar.saltar_Armature_saltar" true))

(event `AnimacionesAleatorias`
  (bind _animaciones (`self.animaciones`))
  (`SkeletalMeshComponent.PlayAnimation` (`self.Mesh`) (`|GetArrayItem` _animaciones (`KismetMathLibrary.RandomInteger` (`KismetArrayLibrary.Array_Length` _animaciones))) true)
  (`self.Stop animation`))

(fn `Play animation`
  (params (Animation :type "AnimationAsset Object Reference") (`Should loop?` :type Boolean))
  (`SkeletalMeshComponent.PlayAnimation` (`self.Mesh`) Animation `Should loop?`))

(fn `Stop animation`
  (bind _mesh (`self.Mesh`))
  (`SkeletalMeshComponent.SetAnimationMode` _mesh "AnimationBlueprint")
  (`SkeletalMeshComponent.SetAnimInstanceClass` _mesh null))

(fn `UserConstructionScript`)